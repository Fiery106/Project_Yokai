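; BP_FastEnemy is an AI enemy, a child Blueprint that runs parent logic and looks up its worth on BeginPlay via its controller.
; Its AttackRange component sets the Blackboard CanAttack key when an actor tagged Barrier enters, and clears it when one leaves.
; Incoming damage is forwarded to TakeDamage along with the damage causer.
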(event OnComponentBeginOverlap(AttackRange)
  (params (OverlappedComponent :type Primitive%20Component%20Object%20Reference) (OtherActor :type Actor%20Object%20Reference) (OtherComp :type Primitive%20Component%20Object%20Reference) (OtherBodyIndex :type Integer) (bFromSweep :type Boolean) (SweepResult :type Hit%20Result%20Structure%20%28by%20ref%29))
  (bind _returnvalue (Pawn|GetController))
  (bind _returnvalue_2 (AI|GetBlackboard _returnvalue))
  ;[0.03125 1 0] Update Blackboard Key value when somthing the AI can attack enters or leaves its attack range
  ;;[1 0.3516 0] Update when something enters it's attack range
  (if (Actor|ActorHasTag OtherActor "Barrier")
    (Utilities|IsValid _returnvalue_2
      (:Is%20Valid
        (AI|Components|Blackboard|SetValueasBool _returnvalue_2 (Utilities|Name|MakeLiteralName "CanAttack") true)))))

(event OnComponentEndOverlap(AttackRange)
  (params (OverlappedComponent :type Primitive%20Component%20Object%20Reference) (OtherActor :type Actor%20Object%20Reference) (OtherComp :type Primitive%20Component%20Object%20Reference) (OtherBodyIndex :type Integer))
  (bind _returnvalue (Pawn|GetController))
  (bind _returnvalue_2 (AI|GetBlackboard _returnvalue))
  ;[0.03125 1 0] Update Blackboard Key value when somthing the AI can attack enters or leaves its attack range
  ;;[0 0.2244 1] Update when something leaves it's attack range
  (if (Actor|ActorHasTag OtherActor "Barrier")
    (Utilities|IsValid _returnvalue_2
      (:Is%20Valid
        (AI|Components|Blackboard|SetValueasBool _returnvalue_2 (Utilities|Name|MakeLiteralName "CanAttack") false)))))

(event EventBeginPlay
  ;[0.8281 0 1] Event Begin Play
  ;;[0 1 0.7188] Do parents Begin play
  (|CallParentFunction)
  ;;[1 0.07031 0] Get your Worth in Mon
  (CallFunction|GetWorth (Pawn|GetController)))

(event Collision|EventActorBeginOverlap
  (params (OtherActor :type Actor%20Object%20Reference))
  (|CallParentFunction OtherActor))

(event EventTick
  (params (DeltaSeconds :type Float%20%28single-precision%29))
  (|CallParentFunction DeltaSeconds))

(event Game|Damage|EventAnyDamage
  (params (Damage :type Float%20%28single-precision%29) (DamageType :type Damage%20Type%20Object%20Reference) (InstigatedBy :type Controller%20Object%20Reference) (DamageCauser :type Actor%20Object%20Reference))
  ;[0 1 0.5547] Take damage
  (CallFunction|TakeDamage Damage DamageCauser))

(fn ConstructionScript
  (|CallParentFunction))