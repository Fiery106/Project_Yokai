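; Parent character for AI enemies, holding health and a cash worth that GetWorth picks from the controller type.
; TakeDamage subtracts health and, on death, reports worth and the kill to the GameMode before destroying the actor.
; Surviving hits reset the forget timer under certain sight conditions, toggling Blackboard chase keys for player hits during cooldown.
; Some writes use a misspelled "CasSeePlayer" key, and the Elite worth branch repeats the Fast controller check, making it unreachable.
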(event EventBeginPlay
  (Variables|Default|SetHealth (Variables|Default|GetMaxHealth)))

(fn ConstructionScript)

(fn TakeDamage
  (params (Damage :type Float%20%28double-precision%29) (Damage%20Dealer :type Actor%20Object%20Reference))
  ;[0.7853 0.9183 1] Take Damage
  ;;[0 0.4375 1] When Hit remove damage taken from health
  (Variables|Default|SetHealth (- (Variables|Default|GetHealth) Damage))
  (if (<= (Variables|Default|GetHealth) 0.0)
    (Class|BPIHUD|UpdateCash(Message) (Game|GetGameMode) (Variables|Default|GetWorth))
    (Class|BPIHUD|EnemyDied(Message) (Game|GetGameMode))
    (Actor|DestroyActor)
    (else
      ;;[0.7088 1 0.1779] If the AI is chasing the player or they have just forgotten them. dealing damage to them will reset the "PlayerSightCooldown" boolean and reset the forget timer. We also set "CanSeePlayer" and "ChasingPlayer" to false and then agian to True, we do this incase the player is already visable to the AI, then setting them to false and the true will update the perception
      (if (or (and (Actor|ActorHasTag Damage%20Dealer "Player") (ScalableFloat|GetValueasBool (AI|GetBlackboard (AI|GetAIController self)) (Utilities|Name|MakeLiteralName "PlayerSightCooldown"))) false)
        (Utilities|FlowControl|Sequence
          (:then_0
            (AI|Components|Blackboard|SetValueasBool (AI|GetBlackboard (AI|GetAIController self)) (Utilities|Name|MakeLiteralName "CasSeePlayer") false)
            (AI|Components|Blackboard|SetValueasBool (AI|GetBlackboard (AI|GetAIController self)) (Utilities|Name|MakeLiteralName "ChasingPlayer") false)
            (AI|Components|Blackboard|SetValueasBool (AI|GetBlackboard (AI|GetAIController self)) (Utilities|Name|MakeLiteralName "PlayerSightCooldown") false)
            (Variables|Default|SetIntegerTimer 0))
          (:then_1
            (AI|Components|Blackboard|SetValueasBool (AI|GetBlackboard (AI|GetAIController self)) (Utilities|Name|MakeLiteralName "CasSeePlayer") true)
            (AI|Components|Blackboard|SetValueasBool (AI|GetBlackboard (AI|GetAIController self)) (Utilities|Name|MakeLiteralName "ChasingPlayer") true)))
        (else
          ;;[1 0 0.01872] Reset Cooldown if the AI is hurt while it is chasing the player
          (if (ScalableFloat|GetValueasBool (AI|GetBlackboard (AI|GetAIController self)) (Utilities|Name|MakeLiteralName "CanSeePlayer"))
            (AI|Components|Blackboard|SetValueasBool (AI|GetBlackboard (AI|GetAIController self)) (Utilities|Name|MakeLiteralName "PlayerSightCooldown") false)
            (Variables|Default|SetIntegerTimer 0)))))))

(fn GetWorth
  (params (Controller :type Controller%20Object%20Reference))
  ;[0.3828 0 1] Set the worth based on the enemy type
  (if (== Controller "/Game/AI/MeleeEnemy/AIC_MeleeEnemy.AIC_MeleeEnemy")
    (Variables|Default|SetWorth (LocalVariables|GetMeleeEnemyWorth))
    (elif (== Controller "/Game/AI/RangedEnemy/AIC_RAngedEnemy.AIC_RangedEnemy")
      (Variables|Default|SetWorth (LocalVariables|GetRangedEnemyWorth))
      (elif (== Controller "/Game/AI/FastEnemy/AIC_FastEnemy.AIC_FastEnemy")
        (Variables|Default|SetWorth (LocalVariables|GetFastEnemyWorth))
        (elif (== Controller "/Game/AI/FastEnemy/AIC_FastEnemy.AIC_FastEnemy")
          (Variables|Default|SetWorth (LocalVariables|GetEliteEnemyWorth)))))))