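; Parent character for AI enemies, handling path assignment, damage, death and per-type stats.
; On BeginPlay it finds the nearest BP_AISpawner and picks a random BP_SplinePath starting at that spawner's number.
; TakeDamage applies brief timed invincibility, reports cash and death to the game mode, or resets blackboard chase and sight-cooldown keys on surviving enemies.
; Setters store type, max health and worth for Melee, Ranged, Fast and Elite controller classes.
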(event EventBeginPlay
  (Utilities|FlowControl|Sequence
    (:then_0
      ;[0 0 0] Find what spawner you spawned at
      (bind _outactors (Actor|GetAllActorsOfClass "/Game/AI/BP/Spawer/BP_AISpawner.BP_AISpawner_C"))
      (for (_array_element _array_index) _outactors
        (if (< (Math|Vector|Distance(Vector) (Transformation|GetActorLocation _array_element) (Transformation|GetActorLocation)) (Variables|Default|GetShortestDistance))
          (Variables|Default|SetShortestDistance (Math|Vector|Distance(Vector) (Transformation|GetActorLocation _array_element) (Transformation|GetActorLocation)))
          (Variables|Default|SetSpawnerIndex _array_index)))
      (Variables|Default|SetSpawner (Variables|/Game/AI/BP/Spawer/BP_AISpawner.BP_AISpawner_C|GetSpawnerNumber (Utilities|Array|Get(acopy) _outactors (Variables|Default|GetSpawnerIndex)))))
    (:then_1
      ;[0.2812 0.0155 0.07767] Get a random spline that starts at the spawner you spawned at
      (bind _outactors_2 (Actor|GetAllActorsOfClass "/Game/AI/Navigation/BP_SplinePath.BP_SplinePath_C"))
      (for _array_element_2 _outactors_2
        (if (Utilities|Enum|Equal(Enum) (Variables|/Game/AI/Navigation/BP_SplinePath.BP_SplinePath_C|GetSplineSpawnerStart _array_element_2) (Variables|Default|GetSpawner))
          (Utilities|Array|Add (Variables|Default|GetValidSplines) _array_element_2)))
      (Variables|Default|SetMySpline (Utilities|Array|Get(acopy) (Variables|Default|GetValidSplines) (Math|Random|RandomIntegerinRange 0 (Utilities|Array|LastIndex (Variables|Default|GetValidSplines))))))))

(fn ConstructionScript)

(fn TakeDamage
  (params (Damage :type Float%20%28double-precision%29) (Damage%20Dealer :type Actor%20Object%20Reference))
  ;[0.7853 0.9183 1] Take Damage
  ;;[0 0.4375 1] When Hit remove damage taken from health
  (if (not (Variables|Default|GetInvinceble))
    (Variables|Default|SetInvinceble true)
    (Utilities|Time|SetTimerbyFunctionName 0 "InvincebilityTimer" 0.5)
    (Variables|Default|SetHealth (- (Variables|Default|GetHealth) Damage))
    (if (<= (Variables|Default|GetHealth) 0.0)
      (Class|BPIHUD|UpdateCash(Message) (Game|GetGameMode) (Variables|Default|GetWorth))
      (Class|BPIHUD|EnemyDied(Message) (Game|GetGameMode))
      (Actor|DestroyActor)
      (else
        (Utilities|IsValid Damage%20Dealer
          (:Is%20Valid
            ;;[0.7088 1 0.1779] If the AI is chasing the player or they have just forgotten them. dealing damage to them will reset the "PlayerSightCooldown" boolean and reset the forget timer. We also set "CanSeePlayer" and "ChasingPlayer" to false and then agian to True, we do this incase the player is already visable to the AI, then setting them to false and the true will update the perception
            (if (or (and (Actor|ActorHasTag Damage%20Dealer "Player") (ScalableFloat|GetValueasBool (AI|GetBlackboard (AI|GetAIController self)) (Utilities|Name|MakeLiteralName "PlayerSightCooldown"))) false)
              (Utilities|FlowControl|Sequence
                (:then_0
                  (AI|Components|Blackboard|SetValueasBool (AI|GetBlackboard (AI|GetAIController self)) (Utilities|Name|MakeLiteralName "CasSeePlayer") false)
                  (AI|Components|Blackboard|SetValueasBool (AI|GetBlackboard (AI|GetAIController self)) (Utilities|Name|MakeLiteralName "ChasingPlayer") false)
                  (AI|Components|Blackboard|SetValueasBool (AI|GetBlackboard (AI|GetAIController self)) (Utilities|Name|MakeLiteralName "PlayerSightCooldown") false)
                  (Variables|Default|SetIntegerTimer 0))
                (:then_1
                  (AI|Components|Blackboard|SetValueasBool (AI|GetBlackboard (AI|GetAIController self)) (Utilities|Name|MakeLiteralName "CasSeePlayer") true)
                  (AI|Components|Blackboard|SetValueasBool (AI|GetBlackboard (AI|GetAIController self)) (Utilities|Name|MakeLiteralName "ChasingPlayer") true)))
              (else
                ;;[1 0 0.01872] Reset Cooldown if the AI is hurt while it is chasing the player
                (if (ScalableFloat|GetValueasBool (AI|GetBlackboard (AI|GetAIController self)) (Utilities|Name|MakeLiteralName "CanSeePlayer"))
                  (AI|Components|Blackboard|SetValueasBool (AI|GetBlackboard (AI|GetAIController self)) (Utilities|Name|MakeLiteralName "PlayerSightCooldown") false)
                  (Variables|Default|SetIntegerTimer 0))))))))))

(fn SetEnemyType
  (params (AI_Controller :type AI%20Controller%20Class%20Reference))
  ;[0 1 0.0628] Set the enemy type to be the AI controller
  (if (== AI_Controller "/Game/AI/Enemies/MeleeEnemy/AIC_MeleeEnemy.AIC_MeleeEnemy_C")
    (Variables|Default|SetEnemyType AI_Controller)
    (elif (== AI_Controller "/Game/AI/Enemies/RangedEnemy/AIC_RangedEnemy.AIC_RangedEnemy_C")
      (Variables|Default|SetEnemyType AI_Controller)
      (elif (== AI_Controller "/Game/AI/Enemies/FastEnemy/AIC_FastEnemy.AIC_FastEnemy_C")
        (Variables|Default|SetEnemyType AI_Controller)
        (elif (== AI_Controller "/Game/AI/Enemies/EliteEnemy/AIC_EliteEnemy.AIC_EliteEnemy_C")
          (Variables|Default|SetEnemyType AI_Controller))))))

(fn SetMaxHealth
  (params (MyMaxHealth :type Float%20%28double-precision%29))
  (bind _enemytype (Variables|Default|GetEnemyType))
  ;[0 0.4635 0.2403] Set Health based on what enemy type you are
  (if (== _enemytype "/Game/AI/Enemies/MeleeEnemy/AIC_MeleeEnemy.AIC_MeleeEnemy_C")
    (Variables|Default|SetMaxHealth MyMaxHealth)
    (elif (== _enemytype "/Game/AI/Enemies/RangedEnemy/AIC_RangedEnemy.AIC_RangedEnemy_C")
      (Variables|Default|SetMaxHealth MyMaxHealth)
      (elif (== _enemytype "/Game/AI/Enemies/FastEnemy/AIC_FastEnemy.AIC_FastEnemy_C")
        (Variables|Default|SetMaxHealth MyMaxHealth)
        (elif (== _enemytype "/Game/AI/Enemies/EliteEnemy/AIC_EliteEnemy.AIC_EliteEnemy_C")
          (Variables|Default|SetMaxHealth MyMaxHealth))))))

(fn SetWorth
  (params (MyWorth :type Integer))
  (bind _enemytype (Variables|Default|GetEnemyType))
  ;[0.2233 0.276 0.2097] Set worth based on what enemy type you are
  (if (== _enemytype "/Game/AI/Enemies/MeleeEnemy/AIC_MeleeEnemy.AIC_MeleeEnemy_C")
    (Variables|Default|SetWorth MyWorth)
    (elif (== _enemytype "/Game/AI/Enemies/RangedEnemy/AIC_RangedEnemy.AIC_RangedEnemy_C")
      (Variables|Default|SetWorth MyWorth)
      (elif (== _enemytype "/Game/AI/Enemies/FastEnemy/AIC_FastEnemy.AIC_FastEnemy_C")
        (Variables|Default|SetWorth MyWorth)
        (elif (== _enemytype "/Game/AI/Enemies/EliteEnemy/AIC_EliteEnemy.AIC_EliteEnemy_C")
          (Variables|Default|SetWorth MyWorth))))))

(fn InvincebilityTimer
  (Variables|Default|SetInvinceble false))