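; Melee enemy AI character that attacks the player and barriers, registering its type, health and worth with its parent class.
; Attack plays a random montage whose "Trace" notify drives a fast looping timer, sphere-tracing weapon points between previous and current positions.
; A DoOnce limits damage to one hit per attack, resetting when the montage completes and notifies the attack task.
; An Elite-enemy buff swaps attack damage and toggles state text.
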(event Custom|TraceHits
  ;[1 0 0.8906] Attack
  ;;[0.07462 1 0.09289] Before we trace the attack we set the last known loc to be the current to stop the trace from going from the last place where the AI attacked
  (for (_array_element _array_index) (Variables|Default|GetTracePoints)
    (Utilities|Array|SetArrayElem (Variables|Default|GetTracePointLocations) _array_index (Transformation|GetWorldLocation _array_element)))
  (bind _returnvalue (Utilities|Time|SetTimerbyEvent (EventDispatchers|CreateEvent :!event Custom|TickTrace) 0.0025 true))
  (Variables|Default|SetAttackTraceTimer _returnvalue))

(event Custom|TracePointArray
  ;[1 0 0.8906] Attack
  ;;[0 0.02733 1] Create an array of the points with which we trace from
  (Variables|Default|SetTracePoints (Utilities|Array|MakeArray (Variables|Default|GetTracePointTip) (Variables|Default|GetTracePointMiddle))))

(event Custom|TickTrace
  ;[1 0 0.8906] Attack
  ;;[0 0.8125 1] Trace from last known loc to currnet loc
  (for (_array_element _array_index) (Variables|Default|GetTracePoints)
    (bind (_outhit _returnvalue) (Collision|SphereTraceByChannel (Utilities|Array|Get(acopy) (Variables|Default|GetTracePointLocations) _array_index) (Transformation|GetWorldLocation _array_element) 15.0 "TraceTypeQuery2" false 0 "None"))
    (Utilities|Array|SetArrayElem (Variables|Default|GetTracePointLocations) _array_index (Transformation|GetWorldLocation _array_element))
    ;;[0 0 0] If we hit something that can take damage, we apply damage
    (if _returnvalue
      (if (or (Actor|ActorHasTag (.HitActor (Collision|BreakHitResult _outhit)) "Player") (Actor|ActorHasTag (.HitActor (Collision|BreakHitResult _outhit)) "Barrier"))
        (Utilities|FlowControl|DoOnce false
          (:Completed
            (Game|Damage|ApplyDamage (.HitActor (Collision|BreakHitResult _outhit)) (Variables|Default|GetAttackDamage) 0 self "/Script/Engine.DamageType")))))))

(event Custom|EnableDamaging
  ;[1 0 0.8906] Attack
  ;;[0 0 0] If we hit something that can take damage, we apply damage
  (Utilities|FlowControl|DoOnce false) ; enters at Reset
)

(event EventBeginPlay
  ;[0.1953 1 0] Event Begin Play
  ;;[1 0.6064 0] Set my enemy type on the parent
  (CallFunction|SetEnemyType (Utilities|GetClass (AI|GetAIController self)))
  (CallFunction|SetMaxHealth (Variables|Default|GetMeleeMaxHealth))
  (CallFunction|SetWorth (Variables|Default|GetMeleeEnemyWorth))
  (|CallParentFunction)
  (CallFunction|TracePointArray))

(event EventBuff
  (params (Buffed? :type Boolean))
  ;[0.2144 0.1533 0.2604] When this AI recive the buff from being near the Elite Enemy
  (if Buffed?
    ;[0.1953 1 0] Event Begin Play
    (Variables|Default|SetAttackDamage (Variables|Default|GetBuffDamage))
    (Rendering|SetVisibility (Variables|Default|GetStateText) true false)
    (else
      (Variables|Default|SetAttackDamage (Variables|Default|GetBaseDamage))
      (Rendering|SetVisibility (Variables|Default|GetStateText) false false))))

(event EventAttack
  (params (AttackTaskRef :type BT%20Task%20Blueprint%20Base%20Object%20Reference))
  ;[1 0 0.8906] Attack
  ;;[1 0.9358 0] When the attack starts we play the montage and based on if the notify envent is ending or starting we trace or stop tracing
  (bind _notifyname (Animation|Montage|PlayMontage (Variables|Character|GetMesh) (Utilities|Array|Get(acopy) (Variables|Default|GetAttackAnims) (Math|Random|RandomIntegerinRange 0 1)))
    (:OnCompleted
      (CallFunction|EnableDamaging)
      (Class|BPIAIComunication|AttackDone(Message) AttackTaskRef))
    (:OnNotifyBegin
      (if (== _notifyname "Trace")
        (CallFunction|TraceHits)))
    (:OnNotifyEnd
      (if (== _notifyname "Trace")
        (Utilities|Time|ClearandInvalidateTimerbyHandle (Variables|Default|GetAttackTraceTimer))))))

(event Game|Damage|EventAnyDamage
  (params (Damage :type Float%20%28single-precision%29) (DamageType :type Damage%20Type%20Object%20Reference) (InstigatedBy :type Controller%20Object%20Reference) (DamageCauser :type Actor%20Object%20Reference))
  ;[1 0 0.2578] Take Damage
  (CallFunction|TakeDamage Damage DamageCauser (AI|GetBlackboard 0)))

(event EventTick
  (params (DeltaSeconds :type Float%20%28single-precision%29))
  ;[0.9624 1 0.9648] Optimizing test
)

(fn ConstructionScript
  (|CallParentFunction))