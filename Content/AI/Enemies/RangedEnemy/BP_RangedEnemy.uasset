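; Ranged enemy Blueprint that specializes a parent enemy class, which supplies the shared behavior.
; On BeginPlay it passes its AI controller's class as the enemy type, plus ranged-specific max health and worth, before running the parent's setup.
; Each tick it copies the actor's rotation to the controller's control rotation.
; Any damage received is forwarded to TakeDamage with the damage causer as dealer.
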(event EventBeginPlay
  ;[1 0.1172 0] Event Begin Play
  ;;[1 0.9643 0.9439] Set My Enemy Type on the Parent
  (CallFunction|SetEnemyType (Utilities|GetClass (AI|GetAIController self)))
  (CallFunction|SetMaxHealth (Variables|Default|GetRangedMaxHealth))
  (CallFunction|SetWorth (Variables|Default|GetRangedEnemyWorth))
  (|CallParentFunction))

(event Collision|EventActorBeginOverlap
  (params (OtherActor :type Actor%20Object%20Reference))
  (|CallParentFunction OtherActor))

(event EventTick
  (params (DeltaSeconds :type Float%20%28single-precision%29))
  (|CallParentFunction DeltaSeconds)
  (Pawn|SetControlRotation (Pawn|GetController) (Transformation|GetActorRotation)))

(event Game|Damage|EventAnyDamage
  (params (Damage :type Float%20%28single-precision%29) (DamageType :type Damage%20Type%20Object%20Reference) (InstigatedBy :type Controller%20Object%20Reference) (DamageCauser :type Actor%20Object%20Reference))
  ;[1 0.6064 0] Take Damage
  (CallFunction|TakeDamage Damage DamageCauser))

(fn ConstructionScript
  (|CallParentFunction))