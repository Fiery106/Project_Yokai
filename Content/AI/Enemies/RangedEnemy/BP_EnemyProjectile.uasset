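; Projectile for the ranged enemy that damages the player and barriers on impact.
; The sphere component's hit event checks the hit actor's tags and uses ApplyDamage on Player or Barrier actors, then destroys the projectile.
; Hits on other valid actors destroy it after a short delay, and a BeginPlay timeout removes any projectile still alive after its lifetime.
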(event OnComponentHit(Sphere)
  (params (HitComponent :type Primitive%20Component%20Object%20Reference) (OtherActor :type Actor%20Object%20Reference) (OtherComp :type Primitive%20Component%20Object%20Reference) (NormalImpulse :type Vector :default "0, 0, 0") (Hit :type Hit%20Result%20Structure%20%28by%20ref%29))
  ;[0.2865 0.2865 0.2865] If the projectile hits somone or something, We send them a interface to damage them and then we delete the actor
  (Utilities|IsValid OtherActor
    (:Is%20Valid
      (if (or (Actor|ActorHasTag OtherActor "Player") (Actor|ActorHasTag OtherActor "Barrier"))
        (Game|Damage|ApplyDamage OtherActor (Variables|Default|GetDamage) 0 0 "/Script/Engine.DamageType")
        (else
          (Utilities|FlowControl|Delay 2.0)))
      (Actor|DestroyActor))))

(event EventBeginPlay
  ;[0.2865 0 0] If the projectile has not hit somthing within 10 seconds, we destroy it
  (Utilities|FlowControl|Delay 1e+01)
  (Actor|DestroyActor))

(fn ConstructionScript)