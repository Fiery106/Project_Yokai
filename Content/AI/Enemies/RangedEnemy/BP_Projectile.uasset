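; Arrow projectile for the ranged enemy, launched toward a predicted target location and dealing damage on impact.
; ShootArrow enables physics on the Arrow and applies an arced launch velocity from SuggestProjectileVelocityCustomArc as an impulse.
; Each tick, a short line trace along the velocity detects hits, sends DamageMessage to Player or Barrier tagged actors, and destroys the projectile.
; It also self-destroys after a timeout if nothing is hit.
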(event EventBeginPlay
  ;[0.2865 0.2865 0.2865] If the projectile has not hit somthing within 10 seconds, we destroy it
  (Utilities|FlowControl|Delay 1e+01)
  (Actor|DestroyActor))

(event EventShootArrow
  (params (PredictedLocation :type Vector :default "0, 0, 0"))
  ;[0.2865 0.2865 0.2865] We add an impulse to the projectile
  (Physics|SetSimulatePhysics (Variables|Default|GetArrow) true)
  (bind _outlaunchvelocity (Game|SuggestProjectileVelocityCustomArc (Transformation|GetActorLocation) PredictedLocation 0.0 0.7))
  (Physics|AddImpulse (Variables|Default|GetArrow) _outlaunchvelocity "None" true))

(event EventTick
  (params (DeltaSeconds :type Float%20%28single-precision%29))
  (bind _arrow (Variables|Default|GetArrow))
  (bind _returnvalue (Transformation|GetWorldLocation _arrow))
  ;[0.2865 0.2865 0.2865] We trace infront of the projectile to check if we hit something, if we do, we destroy the actor and send a signal to who we hit
  (bind (_outhit _returnvalue_2) (Collision|LineTraceByChannel _returnvalue (+ _returnvalue (* (Math|Vector|Normalize (Transformation|GetComponentVelocity _arrow)) 4e+01)) "TraceTypeQuery1" false 0 "ForDuration"))
  (if _returnvalue_2
    (if (or (Actor|ActorHasTag (.HitActor (Collision|BreakHitResult _outhit)) "Barrier") (Actor|ActorHasTag (.HitActor (Collision|BreakHitResult _outhit)) "Player"))
      (Class|BPIDamage|Damage(Message) (.HitActor (Collision|BreakHitResult _outhit)) 1e+01))
    (Actor|DestroyActor)))

(fn ConstructionScript)