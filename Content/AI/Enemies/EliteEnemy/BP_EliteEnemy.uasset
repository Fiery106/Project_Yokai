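; Elite enemy AI character that melee-attacks players and barriers and acts as a buff aura for nearby enemies.
; BeginPlay passes elite type, health and worth to the parent, which also handles incoming damage.
; A placeholder timeline attack swings the weapon, enabling hitbox damage until it finishes and notifies the attack task.
; Entering or leaving the BuffRange sphere toggles other enemies' buff by message.
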(event OnComponentBeginOverlap(BuffRange)
  (params (OverlappedComponent :type Primitive%20Component%20Object%20Reference) (OtherActor :type Actor%20Object%20Reference) (OtherComp :type Primitive%20Component%20Object%20Reference) (OtherBodyIndex :type Integer) (bFromSweep :type Boolean) (SweepResult :type Hit%20Result%20Structure%20%28by%20ref%29))
  ;[1 0.3405 0] When this AI's allies are within the ranged of this collition sphere, we send them a signal and give them a Buff
  (if (Actor|ActorHasTag OtherActor "Enemy")
    (Class|BPIAIComunication|Buff(Message) OtherActor true)))

(event OnComponentEndOverlap(BuffRange)
  (params (OverlappedComponent :type Primitive%20Component%20Object%20Reference) (OtherActor :type Actor%20Object%20Reference) (OtherComp :type Primitive%20Component%20Object%20Reference) (OtherBodyIndex :type Integer))
  ;[1 0.3405 0] When this AI's allies are within the ranged of this collition sphere, we send them a signal and give them a Buff
  (if (Actor|ActorHasTag OtherActor "Enemy")
    (Class|BPIAIComunication|Buff(Message) OtherActor false)))

(event OnComponentBeginOverlap(WeaponHitBox)
  (params (OverlappedComponent :type Primitive%20Component%20Object%20Reference) (OtherActor :type Actor%20Object%20Reference) (OtherComp :type Primitive%20Component%20Object%20Reference) (OtherBodyIndex :type Integer) (bFromSweep :type Boolean) (SweepResult :type Hit%20Result%20Structure%20%28by%20ref%29))
  ;[0.3594 0 1] TEMP - ATTACK
  (if (Variables|Default|GetCanHit)
    (if (or (Actor|ActorHasTag OtherActor "Player") (Actor|ActorHasTag OtherActor "Barrier"))
      (Game|Damage|ApplyDamage OtherActor (Variables|Default|GetBase%20Damage) 0 self "/Script/Engine.DamageType"))))

(event EventBeginPlay
  ;[1 0 0.07031] Event Begin Play
  ;;[0.03125 0 1] Set my enemy type on the parent
  (CallFunction|SetEnemyType (Utilities|GetClass (AI|GetAIController self)))
  (CallFunction|SetMaxHealth (Variables|Default|GetEliteMaxHealth))
  (CallFunction|SetWorth (Variables|Default|GetEliteEnemyWorth))
  (|CallParentFunction)
  (Variables|Default|SetEliteEnemyBlackboard (AI|GetBlackboard 0)))

(event EventAttack
  (params (AttackTaskRef :type BT%20Task%20Blueprint%20Base%20Object%20Reference))
  (bind _weapon (Variables|Default|GetWeapon))
  (bind _relativerotation (Variables|/Script/Engine.SceneComponent|GetRelativeRotation _weapon))
  (bind (_roll _pitch _yaw) (Math|Rotator|BreakRotator _relativerotation))
  ;[0.3594 0 1] TEMP - ATTACK
  (Variables|Default|SetCanHit true)
  (Variables|Default|SetWeaponRotation _relativerotation)
  (bind _swing (Timeline|Timeline PlayFromStart)
    (:Update
      (Transformation|SetRelativeRotation (Variables|Default|GetWeapon) (Math|Rotator|Lerp(Rotator) _relativerotation (Math|Rotator|MakeRotator (- _roll 8.0) _pitch _yaw) _swing) false false))
    (:Finished
      (Transformation|SetRelativeRotation (Variables|Default|GetWeapon) (Variables|Default|GetWeaponRotation) false false)
      (Variables|Default|SetCanHit false)
      (Class|BPIAIComunication|AttackDone(Message) AttackTaskRef))))

(event Game|Damage|EventAnyDamage
  (params (Damage :type Float%20%28single-precision%29) (DamageType :type Damage%20Type%20Object%20Reference) (InstigatedBy :type Controller%20Object%20Reference) (DamageCauser :type Actor%20Object%20Reference))
  ;[0 0.4896 0.1912] Take damage
  (CallFunction|TakeDamage Damage DamageCauser (AI|GetBlackboard 0)))

(event EventTick
  (params (DeltaSeconds :type Float%20%28single-precision%29)))

(fn ConstructionScript
  (|CallParentFunction))