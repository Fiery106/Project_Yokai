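; Fast enemy AI character that sets its own health and worth on the parent class and forwards incoming damage to it.
; Barriers entering or leaving its attack range toggle the CanAttack blackboard key.
; A temporary timeline-driven attack rolls the weapon, enabling its hitbox to damage Player- or Barrier-tagged actors during the swing.
; When the swing ends, it restores the weapon's rotation and notifies the attack task.
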(event OnComponentBeginOverlap(AttackRange)
  (params (OverlappedComponent :type Primitive%20Component%20Object%20Reference) (OtherActor :type Actor%20Object%20Reference) (OtherComp :type Primitive%20Component%20Object%20Reference) (OtherBodyIndex :type Integer) (bFromSweep :type Boolean) (SweepResult :type Hit%20Result%20Structure%20%28by%20ref%29))
  (bind _returnvalue (Pawn|GetController))
  (bind _returnvalue_2 (AI|GetBlackboard _returnvalue))
  ;[0.03125 1 0] Update Blackboard Key value when somthing the AI can attack enters or leaves its attack range
  ;;[1 0.3516 0] Update when something enters it's attack range
  (if (Actor|ActorHasTag OtherActor "Barrier")
    (Utilities|IsValid _returnvalue_2
      (:Is%20Valid
        (AI|Components|Blackboard|SetValueasBool _returnvalue_2 (Utilities|Name|MakeLiteralName "CanAttack") true)))))

(event OnComponentEndOverlap(AttackRange)
  (params (OverlappedComponent :type Primitive%20Component%20Object%20Reference) (OtherActor :type Actor%20Object%20Reference) (OtherComp :type Primitive%20Component%20Object%20Reference) (OtherBodyIndex :type Integer))
  (bind _returnvalue (Pawn|GetController))
  (bind _returnvalue_2 (AI|GetBlackboard _returnvalue))
  ;[0.03125 1 0] Update Blackboard Key value when somthing the AI can attack enters or leaves its attack range
  ;;[0 0.2244 1] Update when something leaves it's attack range
  (if (Actor|ActorHasTag OtherActor "Barrier")
    (Utilities|IsValid _returnvalue_2
      (:Is%20Valid
        (AI|Components|Blackboard|SetValueasBool _returnvalue_2 (Utilities|Name|MakeLiteralName "CanAttack") false)))))

(event OnComponentBeginOverlap(WeaponHitBox)
  (params (OverlappedComponent :type Primitive%20Component%20Object%20Reference) (OtherActor :type Actor%20Object%20Reference) (OtherComp :type Primitive%20Component%20Object%20Reference) (OtherBodyIndex :type Integer) (bFromSweep :type Boolean) (SweepResult :type Hit%20Result%20Structure%20%28by%20ref%29))
  ;[0.2357 0.1972 0.4323] TEMP - ATTACK
  (if (Variables|Default|GetCanHit)
    (if (or (Actor|ActorHasTag OtherActor "Player") (Actor|ActorHasTag OtherActor "Barrier"))
      (Game|Damage|ApplyDamage OtherActor (Variables|Default|GetBase%20Damage) 0 self "/Script/Engine.DamageType"))))

(event EventBeginPlay
  ;[0.8281 0 1] Event Begin Play
  ;;[1 0.07031 0] Set my enemy type on the parent
  (CallFunction|SetEnemyType (Utilities|GetClass (AI|GetAIController self)))
  (CallFunction|SetMaxHealth (Variables|Default|GetFastMaxHealth))
  (CallFunction|SetWorth (Variables|Default|GetFastEnemyWorth))
  (|CallParentFunction))

(event EventAttack
  (params (AttackTaskRef :type BT%20Task%20Blueprint%20Base%20Object%20Reference))
  (bind _weapon (Variables|Default|GetWeapon))
  (bind _relativerotation (Variables|/Script/Engine.SceneComponent|GetRelativeRotation _weapon))
  (bind (_roll _pitch _yaw) (Math|Rotator|BreakRotator _relativerotation))
  ;[0.2357 0.1972 0.4323] TEMP - ATTACK
  (Variables|Default|SetCanHit true)
  (Variables|Default|SetWeaponRotation _relativerotation)
  (bind _swing (Timeline|Timeline PlayFromStart)
    (:Update
      (Transformation|SetRelativeRotation (Variables|Default|GetWeapon) (Math|Rotator|Lerp(Rotator) _relativerotation (Math|Rotator|MakeRotator (- _roll 8.0) _pitch _yaw) _swing) false false))
    (:Finished
      (Transformation|SetRelativeRotation (Variables|Default|GetWeapon) (Variables|Default|GetWeaponRotation) false false)
      (Variables|Default|SetCanHit false)
      (Class|BPIAIComunication|AttackDone(Message) AttackTaskRef))))

(event Game|Damage|EventAnyDamage
  (params (Damage :type Float%20%28single-precision%29) (DamageType :type Damage%20Type%20Object%20Reference) (InstigatedBy :type Controller%20Object%20Reference) (DamageCauser :type Actor%20Object%20Reference))
  ;[0 1 0.5547] Take damage
  (CallFunction|TakeDamage Damage DamageCauser))

(fn ConstructionScript
  (|CallParentFunction))