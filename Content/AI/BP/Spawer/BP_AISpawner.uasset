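; Enemy wave spawner placed as Spawner A, B or C, each marked by its own billboard sprite.
; SpawnWave reads the wave's DT_Waves row and builds a shuffled array from this spawner's melee, ranged, fast and elite counts.
; It reports the total to the game mode, then spawns enemies within its bounds using a delayed-loop macro.
; ChooseBT assigns behavior trees, covering only melee and ranged enemy classes.
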(event EventBeginPlay
  ;[0 0.08594 1] DEBUG
)

(event EventSpawnWave
  (params (WhatWave? :type Integer))
  (bind _returnvalue (Transformation|GetActorLocation))
  (bind _boxextent (Collision|GetActorBounds false false))
  (bind _returnvalue_2 (Math|Random|RandomPointinBoundingBox _returnvalue _boxextent))
  (bind (_x _y) (Class|KismetMathLibrary|BreakVector3f _returnvalue_2))
  ;[0.8516 0 1] Spawn Specified Wave
  (bind _outrownames (DataTable|GetDataTableRowNames "/Game/AI/Spawning/DT_Waves.DT_Waves"))
  (bind _returnvalue_3 (Utilities|GetDataTableRow "/Game/AI/Spawning/DT_Waves.DT_Waves" (Utilities|Array|Get(acopy) _outrownames (- WhatWave? 1)))
    (:then
      ;;[0.3313 1 0] Save as variables for ease of use
      (Variables|Default|SetSpawnerA_Enemies (Utilities|Struct|MakeS_NumberOfEnemies (.meleeenemyclass (.SpawnerA (Utilities|Struct|BreakS_Spawners _returnvalue_3))) (.meleeamount (.SpawnerA (Utilities|Struct|BreakS_Spawners _returnvalue_3))) (.rangedenemyclass (.SpawnerA (Utilities|Struct|BreakS_Spawners _returnvalue_3))) (.rangedamount (.SpawnerA (Utilities|Struct|BreakS_Spawners _returnvalue_3))) (.fastenemyclass (.SpawnerA (Utilities|Struct|BreakS_Spawners _returnvalue_3))) (.fastamount (.SpawnerA (Utilities|Struct|BreakS_Spawners _returnvalue_3))) (.eliteenemyclass (.SpawnerA (Utilities|Struct|BreakS_Spawners _returnvalue_3))) (.eliteamount (.SpawnerA (Utilities|Struct|BreakS_Spawners _returnvalue_3)))))
      (Variables|Default|SetSpawnerB_Enemies (Utilities|Struct|MakeS_NumberOfEnemies (.meleeenemyclass (.SpawnerB (Utilities|Struct|BreakS_Spawners _returnvalue_3))) (.meleeamount (.SpawnerB (Utilities|Struct|BreakS_Spawners _returnvalue_3))) (.rangedenemyclass (.SpawnerB (Utilities|Struct|BreakS_Spawners _returnvalue_3))) (.rangedamount (.SpawnerB (Utilities|Struct|BreakS_Spawners _returnvalue_3))) (.fastenemyclass (.SpawnerB (Utilities|Struct|BreakS_Spawners _returnvalue_3))) (.fastamount (.SpawnerB (Utilities|Struct|BreakS_Spawners _returnvalue_3))) (.eliteenemyclass (.SpawnerB (Utilities|Struct|BreakS_Spawners _returnvalue_3))) (.eliteamount (.SpawnerB (Utilities|Struct|BreakS_Spawners _returnvalue_3)))))
      (Variables|Default|SetSpawnerC_Enemies (Utilities|Struct|MakeS_NumberOfEnemies (.meleeenemyclass (.SpawnerC (Utilities|Struct|BreakS_Spawners _returnvalue_3))) (.meleeamount (.SpawnerC (Utilities|Struct|BreakS_Spawners _returnvalue_3))) (.rangedenemyclass (.SpawnerC (Utilities|Struct|BreakS_Spawners _returnvalue_3))) (.rangedamount (.SpawnerC (Utilities|Struct|BreakS_Spawners _returnvalue_3))) (.fastenemyclass (.SpawnerC (Utilities|Struct|BreakS_Spawners _returnvalue_3))) (.fastamount (.SpawnerC (Utilities|Struct|BreakS_Spawners _returnvalue_3))) (.eliteenemyclass (.SpawnerC (Utilities|Struct|BreakS_Spawners _returnvalue_3))) (.eliteamount (.SpawnerC (Utilities|Struct|BreakS_Spawners _returnvalue_3)))))
      ;;[0.5885 0.7107 1] Based on what spawner this is, we create a array of enemies to spawn
      (switch Utilities|FlowControl|Switch|SwitchonE_SpawnerNumber (Variables|Default|GetSpawnerNumber)
        (:NewEnumerator0
          (CallFunction|MakeEnemyArray (Variables|Default|GetSpawnerA_Enemies)))
        (:NewEnumerator1
          (CallFunction|MakeEnemyArray (Variables|Default|GetSpawnerB_Enemies)))
        (:NewEnumerator2
          (CallFunction|MakeEnemyArray (Variables|Default|GetSpawnerC_Enemies))))
      (Utilities|Array|Shuffle (Variables|Default|GetEnemiesToSpawn))
      ;;[1 0 0.1172] First we tell the game mode how many enemies are being spawned
      (Utilities|FlowControl|Sequence
        (:then_0
          (Variables|Default|SetEnemiesSpawned (Utilities|Array|Length (Variables|Default|GetEnemiesToSpawn)))
          (Class|BPIHUD|EnemiesSpawned(Message) (Game|GetGameMode) (Variables|Default|GetEnemiesSpawned)))
        (:then_1
          ;;[0 1 0.03906] Then we spawn in all the enemies for the wave
          (bind _index (Utilities|ForLoopwithDelay 0 (Utilities|Array|LastIndex (Variables|Default|GetEnemiesToSpawn)) 0.2)
            (:Loop%20Body
              (bind _bt (CallFunction|ChooseBT (Utilities|Array|Get(acopy) (Variables|Default|GetEnemiesToSpawn) _index)))
              (AI|SpawnAIFromClass (Utilities|Array|Get(acopy) (Variables|Default|GetEnemiesToSpawn) _index) _bt (Math|Vector|MakeVector _x _y (.Z (Class|KismetMathLibrary|BreakVector3f _returnvalue))) "0, 0, 0" false 0))
            (:Completed
              (Utilities|Array|Clear (Variables|Default|GetEnemiesToSpawn)))))))))

(fn ConstructionScript
  ;[0.7812 1 0] Set a different sprite for each spawner to show which is which
  (switch Utilities|FlowControl|Switch|SwitchonE_SpawnerNumber (Variables|Default|GetSpawnerNumber)
    (:NewEnumerator0
      (Rendering|Components|Sprite|SetSprite (Variables|Default|GetBillboard) "/Engine/EditorResources/Spawn_Point.Spawn_Point"))
    (:NewEnumerator1
      (Rendering|Components|Sprite|SetSprite (Variables|Default|GetBillboard) "/Engine/EditorResources/Ai_Spawnpoint.Ai_Spawnpoint"))
    (:NewEnumerator2
      (Rendering|Components|Sprite|SetSprite (Variables|Default|GetBillboard) "/Engine/EditorResources/Waypoint.Waypoint"))))

(fn MakeEnemyArray
  (params (Enemies :type S%20Number%20Of%20Enemies%20Structure))
  ;[1 0.02344 0] Add the specified amount of enemies to the array of enemies to spawn
  (if (>= (Variables|Default|GetCounter) (.meleeamount Enemies)) :!label _label
    (Variables|Default|SetCounter 0)
    (if (>= (Variables|Default|GetCounter) (.rangedamount Enemies)) :!label _label_2
      (Variables|Default|SetCounter 0)
      (if (>= (Variables|Default|GetCounter) (.fastamount Enemies)) :!label _label_3
        (Variables|Default|SetCounter 0)
        (if (>= (Variables|Default|GetCounter) (.eliteamount Enemies)) :!label _label_4
          (return)
          (else
            (Math|Integer|IncrementInt (Variables|Default|GetCounter)
              (:%20%20
                (Utilities|Array|Add (Variables|Default|GetEnemiesToSpawn) (.eliteenemyclass Enemies))
                (goto _label_4)))))
        (else
          (Math|Integer|IncrementInt (Variables|Default|GetCounter)
            (:%20%20
              (Utilities|Array|Add (Variables|Default|GetEnemiesToSpawn) (.fastenemyclass Enemies))
              (goto _label_3)))))
      (else
        (Math|Integer|IncrementInt (Variables|Default|GetCounter)
          (:%20%20
            (Utilities|Array|Add (Variables|Default|GetEnemiesToSpawn) (.rangedenemyclass Enemies))
            (goto _label_2)))))
    (else
      (Math|Integer|IncrementInt (Variables|Default|GetCounter)
        (:%20%20
          (Utilities|Array|Add (Variables|Default|GetEnemiesToSpawn) (.meleeenemyclass Enemies))
          (goto _label))))))

(fn ChooseBT
  (params (EnemyClass :type Pawn%20Class%20Reference))
  ;[1 0 0.3984] Based on what enemy is selected we choose it's behaviour tree
  (if (== EnemyClass "/Game/AI/MeleeEnemy/BP_MeleeEnemy.BP_MeleeEnemy_C")
    (bind _output_get (LocalVariables|SetBehaviourTree "/Game/AI/MeleeEnemy/BT_MeleeEnemy.BT_MeleeEnemy"))
    (return _output_get)
    (elif (== EnemyClass "/Game/AI/RangedEnemy/BP_RangedEnemy.BP_RangedEnemy_C")
      (bind _output_get_2 (LocalVariables|SetBehaviourTree "/Game/AI/RangedEnemy/BT_RangedEnemy.BT_RangedEnemy"))
      (return _output_get_2))))