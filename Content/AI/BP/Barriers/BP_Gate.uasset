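; BP_Gate is a destructible barrier actor that AI can perceive and that takes damage when attacked.
; Any damage lowers its current health; at zero it unregisters its perception stimuli source, waits briefly so AI can drop it, then destroys itself.
; The short delay keeps AI from getting stuck on a gate that vanished before unregistering.
; The construction script applies a configurable mesh to the gate.
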(event Game|Damage|EventAnyDamage
  (params (Damage :type Float%20%28single-precision%29) (DamageType :type Damage%20Type%20Object%20Reference) (InstigatedBy :type Controller%20Object%20Reference) (DamageCauser :type Actor%20Object%20Reference))
  ;[0.2865 0.2865 0.2865] When someone attacks the barrier, take damage. If it has no health left, destroy the actor
  (Variables|Default|SetCurrentHealth (- (Variables|Default|GetCurrentHealth) Damage))
  (if (<= (Variables|Default|GetCurrentHealth) 0.0)
    (Class|AIPerceptionStimuliSourceComponent|UnregisterfromPerceptionSystem (Variables|Default|GetAIPerceptionStimuliSource))
    (Utilities|FlowControl|Delay 0.1) ; without the delay the ai does not have time to unregister the gate and will be stuck
    (Actor|DestroyActor)
    (else
      (Development|PrintString (Utilities|String|ToString(Float) (Variables|Default|GetCurrentHealth))))))

(fn ConstructionScript
  ;[0.2865 0.2865 0.2865] Change the mesh of the Barrier
  (Components|StaticMesh|SetStaticMesh (Variables|Default|GetGate) (Variables|Default|GetMesh)))