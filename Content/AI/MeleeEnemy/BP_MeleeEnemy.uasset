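; BP_MeleeEnemy is an AI-controlled melee enemy that can attack players and barriers within its range.
; Overlap events on its Range component set the CanAttack blackboard key true when an actor tagged Player or Barrier enters, and false when any such actor leaves.
; Its Damage event forwards the amount and dealer to TakeDamage, while BeginPlay, Tick, actor overlap and construction defer to the parent class.
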(event OnComponentBeginOverlap(Range)
  (params (OverlappedComponent :type Primitive%20Component%20Object%20Reference) (OtherActor :type Actor%20Object%20Reference) (OtherComp :type Primitive%20Component%20Object%20Reference) (OtherBodyIndex :type Integer) (bFromSweep :type Boolean) (SweepResult :type Hit%20Result%20Structure%20%28by%20ref%29))
  ;[1 0.6064 0] Update Blackboard Key value when somthing the AI can attack enters or leaves its attack range
  ;;[1 0.6064 0] Update when someting enters its attack range
  (if (or (Actor|ActorHasTag OtherActor "Player") (Actor|ActorHasTag OtherActor "Barrier"))
    (AI|Components|Blackboard|SetValueasBool (AI|GetBlackboard (Pawn|GetController)) (Utilities|Name|MakeLiteralName "CanAttack") true)))

(event OnComponentEndOverlap(Range)
  (params (OverlappedComponent :type Primitive%20Component%20Object%20Reference) (OtherActor :type Actor%20Object%20Reference) (OtherComp :type Primitive%20Component%20Object%20Reference) (OtherBodyIndex :type Integer))
  ;[1 0.6064 0] Update Blackboard Key value when somthing the AI can attack enters or leaves its attack range
  ;;[1 0.6064 0] Update ewhen something leaves its attack range
  (if (or (Actor|ActorHasTag OtherActor "Player") (Actor|ActorHasTag OtherActor "Barrier"))
    (AI|Components|Blackboard|SetValueasBool (AI|GetBlackboard (Pawn|GetController)) (Utilities|Name|MakeLiteralName "CanAttack") false)))

(event EventBeginPlay
  (|CallParentFunction))

(event Collision|EventActorBeginOverlap
  (params (OtherActor :type Actor%20Object%20Reference))
  (|CallParentFunction OtherActor))

(event EventTick
  (params (DeltaSeconds :type Float%20%28single-precision%29))
  (|CallParentFunction DeltaSeconds))

(event EventDamage
  (params (Damage :type Float%20%28double-precision%29) (DamageDealer :type Actor%20Object%20Reference))
  ;[1 0.6064 0] Take Damage
  (CallFunction|TakeDamage Damage DamageDealer))

(fn ConstructionScript
  (|CallParentFunction))