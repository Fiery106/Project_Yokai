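; GameMode_Defense is a game mode that creates and controls the player HUD for the Defense game.
; On BeginPlay it caches the game instance and player character, adds the HUD widget to the viewport, and initializes the stamina bar.
; UpdateStamina and WeaponWheel events let the stamina bar be refreshed from the character's Stamina and toggle the radial menu with its background blur.
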(event EventBeginPlay
  (CallFunction|FuncPrerequisites)
  (CallFunction|FuncUpdateStamina))

(event EventWeaponWheel
  (params (Visibility :type Boolean))
  (CallFunction|FuncShowMenu Visibility))

(event EventUpdateStamina
  (CallFunction|FuncUpdateStamina))

(fn ConstructionScript)

(fn FuncPrerequisites
  (bind _asgame_inst_defense (Utilities|Casting|CastToGameInst_Defense (Game|GetGameInstance)))
  (Variables|Default|SetAs%20Game%20Inst%20Defense _asgame_inst_defense)
  (bind _asplayer_character_defense (Utilities|Casting|CastToPlayerCharacter_Defense (Game|Player|GetPlayerPawn 0)))
  (Variables|Default|SetAs%20Player%20Character%20Defense _asplayer_character_defense)
  (bind _returnvalue (UserInterface|CreateWidget "/Game/Widgets/HUD/Widget_HUD.Widget_HUD_C"))
  (bind _output_get (Variables|Default|SetHUD _returnvalue))
  (UserInterface|Viewport|AddtoViewport _output_get 0))

(fn FuncUpdateStamina
  (Progress|SetPercent (Variables|/Game/Widgets/HUD/Widget_Stamina.Widget_Stamina_C|GetStaminaBar (Variables|/Game/Widgets/HUD/Widget_HUD.Widget_HUD_C|GetWidget_Stamina (Variables|Default|GetHUD))) (Variables|/Game/Player/Blueprints/PlayerCharacter_Defense.PlayerCharacter_Defense_C|GetStamina (Variables|Default|GetAs%20Player%20Character%20Defense))))

(fn FuncShowMenu
  (params (visibility :type Boolean))
  (bind _hud (Variables|Default|GetHUD))
  (bind _widget_radialmenu (Variables|/Game/Widgets/HUD/Widget_HUD.Widget_HUD_C|GetWidget_RadialMenu _hud))
  (if visibility
    (Widget|SetVisibility _widget_radialmenu "Visible")
    (else
      (Widget|SetVisibility _widget_radialmenu "Hidden"))))