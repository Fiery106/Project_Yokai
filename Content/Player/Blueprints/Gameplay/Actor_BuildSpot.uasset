(event EventBeginPlay
  ;[0.01133 0.708 0.2671] Changing tags will alter the number of options that can be built on this spot.
  (CallFunction|FuncVisibility true)
  (if (Variables|Default|GetOnPath)
    (Utilities|Array|SetArrayElem (Variables|Actor|GetTags) 2 "Path")))

(event EventConstruct
  (params (Tower%20To%20Build :type Enum_Towers%20Enum :default "NewEnumerator0"))
  ;[0.0358 0.536 0.06213] Building a tower on this spot will hide and occupy this spot
  (if (not (Variables|Default|GetOccupied))
    (Variables|Default|SetOccupied true)
    (CallFunction|FuncVisibility false)))

(event EventSell
  ;[0.5 0.06784 0.01801] Selling the tower will destroy the closest tower located to this building spot, then make it visible and available
  (Variables|Default|SetOccupied false)
  (CallFunction|FuncVisibility true)
  (bind _outactors (Actor|GetAllActorsOfClass "/Game/Towers/Actor_Tower.Actor_Tower_C"))
  (if (not (> (.Distance (Actor|FindNearestActor (Transformation|GetActorLocation) _outactors)) 0.0)) ; Check to make sure it removes the correct tower
    (Actor|DestroyActor (.ReturnValue (Actor|FindNearestActor (Transformation|GetActorLocation) _outactors)))))

(event EventTick
  (params (DeltaSeconds :type Float%20%28single-precision%29))
  (bind _cube (Variables|Default|GetCube))
  ;[0 0.365 0.2829] Disable collisions when the player is not close enough to the building spot (Prevents the player not selecting the right tower to upgrade)
  (bind _outactors (Actor|GetAllActorsOfClass "/Script/Engine.Pawn"))
  (if (Math|Boolean|ANDBoolean (<= (.Distance (Actor|FindNearestActor (Transformation|GetActorLocation) _outactors)) 265.0) (Actor|ActorHasTag (.ReturnValue (Actor|FindNearestActor (Transformation|GetActorLocation) _outactors)) "Player") (not (Variables|Default|GetOccupied)))
    (Collision|SetCollisionEnabled _cube "QueryAndPhysics")
    (else
      (Collision|SetCollisionEnabled _cube "NoCollision"))))

(fn ConstructionScript)

(fn FuncVisibility
  (params (Visible :type Boolean))
  (bind _cube (Variables|Default|GetCube))
  (bind _capsule (Variables|Default|GetCapsule))
  (if Visible
    (Rendering|SetVisibility _cube true false)
    (Collision|SetCollisionEnabled _capsule "QueryAndPhysics")
    (else
      (Rendering|SetVisibility _cube false false)
      (Collision|SetCollisionEnabled _capsule "NoCollision"))))