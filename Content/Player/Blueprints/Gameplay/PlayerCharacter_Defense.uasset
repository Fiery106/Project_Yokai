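; Player character for a tower defense game, handling movement, combat and interaction with build spots, towers and shops.
; A weapon wheel switches between katana (timeline swing, overlap hits), bow (camera-aimed arrow) and musket (capsule-trace headshots, timed reload).
; A capsule trace reads actor tags to open menus, with MenuCheck gating input and the GameMode receiving UI, ammo and health updates.
; Includes coyote-time jumping and debug keys; stamina consumption is never invoked.
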(event OnComponentBeginOverlap(HitDetection)
  (params (OverlappedComponent :type Primitive%20Component%20Object%20Reference) (OtherActor :type Actor%20Object%20Reference) (OtherComp :type Primitive%20Component%20Object%20Reference) (OtherBodyIndex :type Integer) (bFromSweep :type Boolean) (SweepResult :type Hit%20Result%20Structure%20%28by%20ref%29))
  ;[0 0.8594 1] TEMP - Melee attack and hit detection
  ;;[1 0 0.09375] Melee Weapon Hit detection
  (if (Variables|Default|GetAttacking)
    (if (Actor|ActorHasTag OtherActor "Enemy")
      (Game|Damage|ApplyDamage OtherActor (Variables|Default|GetKataneDamage) 0 self "/Script/Engine.DamageType"))))

(event Custom|StopInvincibility
  ;[0.349 0.004114 0.2035] take damage
  (Variables|Default|SetInvinceble false))

(event Custom|ReloadingTimer
  ;[0 0.2969 1] Musket Logic
  (Audio|PlaySoundatLocation "/Engine/VREditor/Sounds/UI/Gizmo_Handle_Clicked.Gizmo_Handle_Clicked" (Transformation|GetWorldLocation (Variables|Default|GetMusket)) "0, 0, 0" 0.1 0.5 0.0 0 0 0 0)
  (Variables|Default|SetMusketReloading? false))

(event Input|EnhancedActionEvents|EnhancedInputActionInput_Attack
  (params (ActionValue :type Boolean) (ElapsedSeconds :type Float%20%28double-precision%29) (TriggeredSeconds :type Float%20%28double-precision%29) (InputAction :type Input%20Action%20Object%20Reference :default "/Game/Player/Input/Input_Attack.Input_Attack"))
  (bind _returnvalue (Game|GetGameMode))
  (bind _currentitem (Variables|Default|GetCurrentItem))
  (bind _katana (Variables|Default|GetKatana))
  (bind _relativerotation (Variables|/Script/Engine.SceneComponent|GetRelativeRotation _katana))
  (bind (_roll _pitch _yaw) (Math|Rotator|BreakRotator _relativerotation))
  (:Started
    (switch Utilities|FlowControl|Switch|SwitchonEnum_EquippedItem (Variables|Default|GetCurrentItem)
      (:NewEnumerator0
        ;[0 0.8594 1] TEMP - Melee attack and hit detection
        (if (not (Variables|Default|GetAttacking))
          (Variables|Default|SetAttacking true)
          (bind _slice (Timeline|Katane PlayFromStart)
            (:Update
              (Transformation|SetRelativeRotation (Variables|Default|GetKatana) (Math|Rotator|Lerp(Rotator) _relativerotation (Math|Rotator|MakeRotator _roll _pitch (- _yaw 1e+01)) _slice) false false))
            (:Finished
              (Utilities|FlowControl|Delay 0.4)
              (Transformation|SetRelativeRotation (Variables|Default|GetKatana) (Variables|Default|GetKataneRotation) false false)
              (Variables|Default|SetAttacking false)))))
      (:NewEnumerator1
        (bind _hasenough (Class|BPIHUD|UseAmmo(Message) _returnvalue _currentitem))
        (if _hasenough
          ;[0.09883 0.4531 0.08159] Bow Logic
          (CallFunction|FuncBowAttack)))
      (:NewEnumerator2
        ;[0 0.2969 1] Musket Logic
        (if (not (Variables|Default|GetMusketReloading?))
          (Variables|Default|SetMusketReloading? true)
          (bind _hasenough_2 (Class|BPIHUD|UseAmmo(Message) _returnvalue _currentitem))
          (if _hasenough_2
            (Utilities|Time|SetTimerbyEvent (delegate Custom|ReloadingTimer) 1.0)
            (CallFunction|FuncMusketShot)))))))

(event Input|EnhancedActionEvents|EnhancedInputActionInput_Tab
  (params (ActionValue :type Boolean) (ElapsedSeconds :type Float%20%28double-precision%29) (TriggeredSeconds :type Float%20%28double-precision%29) (InputAction :type Input%20Action%20Object%20Reference :default "/Game/Player/Input/Input_Tab.Input_Tab"))
  (bind _returnvalue (Viewport|GetViewportSize))
  (bind _returnvalue_2 (/ _returnvalue "(X=2.800000,Y=2.000000)"))
  ;[0.1714 0.01938 0] Open wheel selection menu
  (:Triggered
    (if (not (Utilities|Enum|Equal(Enum) (Variables|Default|GetMenuCheck) "NewEnumerator0"))
      (Variables|Default|SetMenuCheck "NewEnumerator0")
      (Class|BPIHUD|WeaponWheel(Message) (Game|GetGameMode) true)))
  (:Started
    (Class|PlayerController|SetMouseLocation (Game|GetPlayerController 0) (Math|Float|Truncate (.x _returnvalue_2)) (Math|Float|Truncate (.y _returnvalue_2))))
  (:Completed
    (Class|BPIHUD|WeaponWheel(Message) (Game|GetGameMode) false)
    (Utilities|FlowControl|Delay 0.5)
    (Variables|Default|SetMenuCheck "NewEnumerator3")
    ;[0.1615 0.04039 0.005886] Zoom in with ranged weapon
    (Utilities|FlowControl|Sequence
      (:then_0
        (Variables|/Script/Engine.CharacterMovementComponent|SetMaxWalkSpeed (Variables|Character|GetCharacterMovement) (Variables|Default|GetSpeed)))
      (:then_1
        (Class|BPIHUD|AddCrosshair(Message) (Game|GetGameMode) false))
      (:then_2
        (Utilities|FlowControl|RetriggerableDelay 0.5) ; Mash prevention
        (Variables|Default|SetZoomedIn false)))))

(event Input|EnhancedActionEvents|EnhancedInputActionInput_Special
  (params (ActionValue :type Boolean) (ElapsedSeconds :type Float%20%28double-precision%29) (TriggeredSeconds :type Float%20%28double-precision%29) (InputAction :type Input%20Action%20Object%20Reference :default "/Game/Player/Input/Input_Special.Input_Special"))
  (bind _charactermovement (Variables|Character|GetCharacterMovement))
  (bind _speed (Variables|Default|GetSpeed))
  (bind _menucheck (Variables|Default|GetMenuCheck))
  (bind _currentitem (Variables|Default|GetCurrentItem))
  (bind _returnvalue (Utilities|Enum|Equal(Enum) _currentitem "NewEnumerator1"))
  (bind _returnvalue_2 (Utilities|Enum|Equal(Enum) _menucheck "NewEnumerator3"))
  (bind _returnvalue_3 (Utilities|Enum|Equal(Enum) _currentitem "NewEnumerator2"))
  (bind _returnvalue_4 (or _returnvalue _returnvalue_3))
  (bind _returnvalue_5 (and _returnvalue_4 _returnvalue_2))
  ;[0.1615 0.04039 0.005886] Zoom in with ranged weapon
  (:Triggered
    (if _returnvalue_5
      (Utilities|FlowControl|Sequence
        (:then_0
          (Variables|/Script/Engine.CharacterMovementComponent|SetMaxWalkSpeed _charactermovement (/ _speed 2.0)))
        (:then_1
          (Class|BPIHUD|AddCrosshair(Message) (Game|GetGameMode) true))
        (:then_2
          (if (Variables|Default|GetZoomedIn)
            (Utilities|FlowControl|RetriggerableDelay 0.1) ; Mash prevention
            (bind _zoomin (Timeline|Timeline Reverse)
              (:Update
                (Variables|/Script/Engine.SpringArmComponent|SetTargetArmLength (Variables|Default|GetSpringArm) (- (Variables|Default|GetTarget%20Arm%20Length) (* _zoomin 1e+02)))))
            (else
              (Variables|Default|SetZoomedIn true)
              (Timeline|Timeline Play)))))
      (elif (Utilities|Enum|Equal(Enum) (Variables|Default|GetCurrentItem) "NewEnumerator0") ; Melee charge attack
        _)))
  (:Completed
    (if _returnvalue_5
      (Utilities|FlowControl|Sequence
        (:then_0
          (Variables|/Script/Engine.CharacterMovementComponent|SetMaxWalkSpeed _charactermovement _speed))
        (:then_1
          (Class|BPIHUD|AddCrosshair(Message) (Game|GetGameMode) false))
        (:then_2
          (Utilities|FlowControl|RetriggerableDelay 0.5) ; Mash prevention
          (Variables|Default|SetZoomedIn false))))))

(event Game|Damage|EventAnyDamage
  (params (Damage :type Float%20%28single-precision%29) (DamageType :type Damage%20Type%20Object%20Reference) (InstigatedBy :type Controller%20Object%20Reference) (DamageCauser :type Actor%20Object%20Reference))
  ;[0.349 0.004114 0.2035] take damage
  (if (not (Variables|Default|GetInvinceble))
    (Variables|Default|SetInvinceble true)
    (Class|BPIHUD|UpdateHealth(Message) (Game|GetGameMode) Damage)
    (Utilities|Time|SetTimerbyEvent (delegate Custom|StopInvincibility) 1.0)
    (if (<= (Variables|Default|GetCurrentHealth) 0.0)
      (Input|SetInputModeUIOnly (Game|GetPlayerController 0) 0 "DoNotLock" false))))

(event EventChangeItem
  (params (NewItem :type Enum_EquippedItem%20Enum :default "NewEnumerator0") (ArrowType :type String))
  ;[0 0.107 0.1559] Change Player State(s) after selecting an item from the weapon wheel
  (Variables|Default|SetCurrentItem NewItem)
  (CallFunction|FuncSetWeaponVisibility))

(event Input|KeyboardEvents|DebugKeyK
  (params (Key :type Key%20Structure) (ActionValue :type Input%20Action%20Value%20Structure))
  ;[0.8962 1 0.6094] DEBUG
  ;;[0.6641 0 1] Kill all enemies
  (:Pressed
    (Utilities|FlowControl|Sequence
      (:then_0
        (bind _outactors (Actor|GetAllActorsOfClass "/Game/AI/Enemies/RangedEnemy/BP_RangedEnemy.BP_RangedEnemy_C"))
        (if (not (Utilities|Array|IsEmpty _outactors))
          (for _array_element _outactors
            (Game|Damage|ApplyDamage _array_element 1e+03 0 self "/Script/Engine.DamageType"))))
      (:then_1
        (bind _outactors_2 (Actor|GetAllActorsOfClass "/Game/AI/Enemies/MeleeEnemy/BP_MeleeEnemy.BP_MeleeEnemy_C"))
        (if (not (Utilities|Array|IsEmpty _outactors_2))
          (for _array_element_2 _outactors_2
            (Game|Damage|ApplyDamage _array_element_2 1e+03 0 self "/Script/Engine.DamageType"))))
      (:then_2
        (bind _outactors_3 (Actor|GetAllActorsOfClass "/Game/AI/Enemies/FastEnemy/BP_FastEnemy.BP_FastEnemy_C"))
        (if (not (Utilities|Array|IsEmpty _outactors_3))
          (for _array_element_3 _outactors_3
            (Game|Damage|ApplyDamage _array_element_3 1e+03 0 self "/Script/Engine.DamageType"))))
      (:then_3
        (bind _outactors_4 (Actor|GetAllActorsOfClass 0))
        (if (Utilities|Array|IsEmpty _outactors_4)
          (for _array_element_4 _outactors_4
            (Game|Damage|ApplyDamage 0 1e+03 0 self "/Script/Engine.DamageType")))))))

(event Input|KeyboardEvents|DebugKeyT
  (params (Key :type Key%20Structure) (ActionValue :type Input%20Action%20Value%20Structure))
  (bind _current_wave (Variables|Default|GetCurrent%20Wave))
  ;[0.8962 1 0.6094] DEBUG
  ;;[1 0.5391 0] Start wave
  (:Pressed
    (Math|Integer|IncrementInt _current_wave
      (:%20%20
        (Class|BPIHUD|WaveStart(Message) (Game|GetGameMode) 5 _current_wave)
        (Variables|Default|SetWaveInProgress true)))))

(event Input|KeyboardEvents|DebugKeyM
  (params (Key :type Key%20Structure) (ActionValue :type Input%20Action%20Value%20Structure))
  ;[0.8962 1 0.6094] DEBUG
  (:Pressed
    (Class|BPIHUD|UpdateCash(Message) (Game|GetGameMode) 200)))

(event OnComponentEndOverlap(InteractRadius)
  (params (OverlappedComponent :type Primitive%20Component%20Object%20Reference) (OtherActor :type Actor%20Object%20Reference) (OtherComp :type Primitive%20Component%20Object%20Reference) (OtherBodyIndex :type Integer))
  (bind _returnvalue (Game|GetGameMode))
  ;[0 0.04977 0.1714] Hide interact prompt when the player stops being near the object
  (if (Utilities|Enum|Equal(Enum) (Variables|Default|GetMenuCheck) "NewEnumerator1")
    (Class|BPIHUD|BuildMenu(Message) _returnvalue false)
    (elif (Utilities|Enum|Equal(Enum) (Variables|Default|GetMenuCheck) "NewEnumerator2")
      (Class|BPIHUD|UpgradeMenu(Message) _returnvalue false (Variables|Default|GetLastSelectedTower))
      (elif (Utilities|Enum|Equal(Enum) (Variables|Default|GetMenuCheck) "NewEnumerator4")
        (Class|BPIHUD|ShopMenu(Message) _returnvalue false))))
  (Class|BPIHUD|InteractPrompt(Message) _returnvalue false) ; Hide the interact prompt and close the build menu
  (Variables|Default|SetMenuCheck "NewEnumerator3"))

(event OnComponentBeginOverlap(InteractRadius)
  (params (OverlappedComponent :type Primitive%20Component%20Object%20Reference) (OtherActor :type Actor%20Object%20Reference) (OtherComp :type Primitive%20Component%20Object%20Reference) (OtherBodyIndex :type Integer) (bFromSweep :type Boolean) (SweepResult :type Hit%20Result%20Structure%20%28by%20ref%29))
  ;[0.000998 0.01574 0.1714] Show interact prompt when an interactible object is interactible
  (if (and (Actor|ActorHasTag OtherActor "Interactible") (Utilities|Enum|Equal(Enum) (Variables|Default|GetMenuCheck) "NewEnumerator3"))
    (Class|BPIHUD|InteractPrompt(Message) (Game|GetGameMode) true) ; When player is within range of an interactible object, show prompt
  ))

(event Custom|CheckFloor
  (bind _charactermovement (Variables|Character|GetCharacterMovement))
  (bind _capsulecomponent (Variables|Collision|GetCapsuleComponent))
  (bind _returnvalue (Transformation|GetWorldLocation _capsulecomponent))
  (bind _floorresult (Pawn|Components|CharacterMovement|FindFloor _charactermovement _returnvalue))
  ;[0.843 0.843 0.843] Check floor every few miliseconds for movement related stuff
  (if (and (.bwalkablefloor _floorresult) (< (.floordist _floorresult) 1e+01))
    (Variables|Default|SetValidDash true)
    (Variables|Default|SetValidJump true)
    (else
      (Utilities|FlowControl|Delay 0.2) ; Coyote time
      (Variables|Default|SetValidJump false))))

(event Custom|StaminaRegen
  ;[0 0.05127 0.1559] Replenish Stamina slowly after not performing an action
  (CallFunction|FuncStaminaRegen (stale EventUpdateStamina _returnvalue))
  (if (== (Variables|Default|GetStamina) 1.0)
    (Utilities|Time|ClearandInvalidateTimerbyHandle (stale EventUpdateStamina _returnvalue))))

(event Input|EnhancedActionEvents|EnhancedInputActionInput_Look
  (params (ActionValue :type Vector%202D%20Structure) (ElapsedSeconds :type Float%20%28double-precision%29) (TriggeredSeconds :type Float%20%28double-precision%29) (InputAction :type Input%20Action%20Object%20Reference :default "/Game/Player/Input/Input_Look.Input_Look"))
  ;[0.1714 0 0.07421] Look around
  (:Triggered
    (Pawn|Input|AddControllerYawInput (.x ActionValue))
    (Pawn|Input|AddControllerPitchInput (* (.y ActionValue) -1.0))))

(event Input|EnhancedActionEvents|EnhancedInputActionInput_Move
  (params (ActionValue :type Vector%202D%20Structure) (ElapsedSeconds :type Float%20%28double-precision%29) (TriggeredSeconds :type Float%20%28double-precision%29) (InputAction :type Input%20Action%20Object%20Reference :default "/Game/Player/Input/Input_Move.Input_Move"))
  ;[0.1714 0.002125 0.1356] Basic Movement
  (:Triggered
    (Pawn|Input|AddMovementInput (Transformation|GetActorRightVector) (.x ActionValue) false)
    (Pawn|Input|AddMovementInput (Transformation|GetActorForwardVector) (.y ActionValue) false)))

(event Input|EnhancedActionEvents|EnhancedInputActionInput_Evade
  (params (ActionValue :type Boolean) (ElapsedSeconds :type Float%20%28double-precision%29) (TriggeredSeconds :type Float%20%28double-precision%29) (InputAction :type Input%20Action%20Object%20Reference :default "/Game/Player/Input/Input_Evade.Input_Evade"))
  (bind _returnvalue (Transformation|GetVelocity))
  ;[0.1651 0.001214 0.1714] Evade Attacks
  (:Started
    (if (Variables|Default|GetValidDash)
      (Variables|Default|SetValidDash false)
      (Character|LaunchCharacter (Math|Vector|MakeVector (* (.x _returnvalue) 1.25) (* (.y _returnvalue) 1.25) 3e+02) false true))))

(event Input|EnhancedActionEvents|EnhancedInputActionInput_Jump
  (params (ActionValue :type Boolean) (ElapsedSeconds :type Float%20%28double-precision%29) (TriggeredSeconds :type Float%20%28double-precision%29) (InputAction :type Input%20Action%20Object%20Reference :default "/Game/Player/Input/Input_Jump.Input_Jump"))
  ;[0.1119 0 0.1714] Basic Jump
  (:Started
    (if (Variables|Default|GetValidJump)
      (Variables|Default|SetValidJump false)
      (Character|LaunchCharacter "0.000000,0.000000,500.000000" false true))))

(event Input|EnhancedActionEvents|EnhancedInputActionInput_Sprint
  (params (ActionValue :type Boolean) (ElapsedSeconds :type Float%20%28double-precision%29) (TriggeredSeconds :type Float%20%28double-precision%29) (InputAction :type Input%20Action%20Object%20Reference :default "/Game/Player/Input/Input_Sprint.Input_Sprint"))
  (bind _speed (Variables|Default|GetSpeed))
  (bind _charactermovement (Variables|Character|GetCharacterMovement))
  ;[0.06663 0 0.1714] Sprint Mechanic
  (:Triggered
    (if (!= (.y (Pawn|Components|CharacterMovement|GetCurrentAcceleration (Variables|Character|GetCharacterMovement))) 0.0)
      (Variables|Default|SetSprinting true)
      (Variables|/Script/Engine.CharacterMovementComponent|SetMaxWalkSpeed _charactermovement (+ (Math|Float|Clamp(Float) (Variables|/Script/Engine.CharacterMovementComponent|GetMaxWalkSpeed _charactermovement) _speed (* _speed 1.6)) 1e+01)) ; Gradually increase player's speed until it reaches the max
      (else
        (Variables|/Script/Engine.CharacterMovementComponent|SetMaxWalkSpeed _charactermovement _speed :!label _label)
        (Variables|Default|SetSprinting false))))
  (:Canceled
    (goto _label))
  (:Completed
    (goto _label)))

(event Input|EnhancedActionEvents|EnhancedInputActionInput_Interact
  (params (ActionValue :type Boolean) (ElapsedSeconds :type Float%20%28double-precision%29) (TriggeredSeconds :type Float%20%28double-precision%29) (InputAction :type Input%20Action%20Object%20Reference :default "/Game/Player/Input/Input_Interact.Input_Interact"))
  (bind _selectedactor_s_ (Variables|Default|GetSelectedActor%28s%29))
  (bind _mesh (Variables|Character|GetMesh))
  (bind _selectedtag (Variables|Default|GetSelectedTag))
  (bind _returnvalue (Transformation|GetWorldLocation _mesh))
  ;[0.11 0 0] Interact with object
  (:Started
    (if (Utilities|Enum|Equal(Enum) (Variables|Default|GetMenuCheck) "NewEnumerator3")
      (bind (_outhit _returnvalue_2) (Collision|CapsuleTraceByChannel _returnvalue _returnvalue (Variables|Default|GetInteract%20Radius) 0.0 "TraceTypeQuery3" false 0 "ForDuration" true "(R=1.000000,G=0.000000,B=0.000000,A=1.000000)" "(R=0.000000,G=1.000000,B=0.000000,A=1.000000)" 1.0))
      ;;[0.2874 0.1413 0.0137] Interact with building spot to build a tower
      (if _returnvalue_2 ; Necessary check to prevent compile error
        (if (and (.bblockinghit _outhit) (Actor|ActorHasTag (.hitactor _outhit) "Build"))
          (bind _output_get (Variables|Default|SetOut%20Hit%20Hit%20Actor (.hitactor _outhit)))
          (Utilities|Array|SetArrayElem (Variables|Default|GetSelectedActor%28s%29) 0 _output_get) ; Building Spot
          (Utilities|Array|SetArrayElem _selectedtag 0 (Utilities|Array|Get(acopy) (Variables|/Script/Engine.Actor|GetTags (Variables|Default|GetOut%20Hit%20Hit%20Actor)) 2)) ; On path or not
          (Variables|Default|SetMenuCheck "NewEnumerator1")
          (Class|BPIHUD|BuildMenu(Message) (Game|GetGameMode) true)
          (CallFunction|FuncCenterMouse))
        ;;[0.3372 0.1746 0.1329] Manage tower to upgrade or sell
        (if (and (.bblockinghit _outhit) (Actor|ActorHasTag (.hitactor _outhit) "Tower"))
          (bind _output_get_2 (Variables|Default|SetOut%20Hit%20Hit%20Actor (.hitactor _outhit)))
          (bind _outactors (Actor|GetAllActorsOfClass "/Game/Player/Blueprints/Gameplay/Actor_BuildSpot.Actor_BuildSpot_C"))
          (Utilities|Array|SetArrayElem _selectedactor_s_ 0 (.ReturnValue (Actor|FindNearestActor (Transformation|GetActorLocation _output_get_2) _outactors))) ; Building Spot
          (Utilities|Array|SetArrayElem _selectedactor_s_ 1 (Variables|Default|GetOut%20Hit%20Hit%20Actor)) ; Set tower to upgrade
          (Utilities|Array|SetArrayElem _selectedtag 1 (Utilities|Array|Get(acopy) (Variables|/Script/Engine.Actor|GetTags (Variables|Default|GetOut%20Hit%20Hit%20Actor)) 4)) ; SellPrice
          (Variables|Default|SetMenuCheck "NewEnumerator2")
          (bind _output_get_3 (Variables|Default|SetLastSelectedTower (Utilities|Array|Get(acopy) (Variables|/Script/Engine.Actor|GetTags (Variables|Default|GetOut%20Hit%20Hit%20Actor)) 3)))
          (Class|BPIHUD|UpgradeMenu(Message) (Game|GetGameMode) true _output_get_3)
          (CallFunction|FuncCenterMouse))
        ;;[0.05127 0.02732 0.0319] Open up the shop menu to buy useful items
        (if (and (.bblockinghit _outhit) (Actor|ActorHasTag (.hitactor _outhit) "Shop"))
          (Variables|Default|SetMenuCheck "NewEnumerator4")
          (Class|BPIHUD|ShopMenu(Message) (Game|GetGameMode) true)
          (CallFunction|FuncCenterMouse))
        (else
          (Class|BPIHUD|UseConsume(Message) (Game|GetGameMode)))))))

(event Input|EnhancedActionEvents|EnhancedInputActionInput_Pause
  (params (ActionValue :type Boolean) (ElapsedSeconds :type Float%20%28double-precision%29) (TriggeredSeconds :type Float%20%28double-precision%29) (InputAction :type Input%20Action%20Object%20Reference :default "/Game/Player/Input/Input_Pause.Input_Pause"))
  (bind _returnvalue (Game|GetGameMode))
  (bind _returnvalue_2 (Game|GetGameMode))
  ;[0.02956 0 0.1714] Set game to paused & Open pause menu
  (:Started
    (if (Utilities|Enum|Equal(Enum) (Variables|Default|GetMenuCheck) "NewEnumerator3")
      (if (Game|IsGamePaused)
        (Game|SetGamePaused false)
        (Class|BPIHUD|PauseMenu(Message) _returnvalue_2 false)
        (else
          (Game|SetGamePaused true)
          (Class|BPIHUD|PauseMenu(Message) _returnvalue_2 true)))
      (else
        ;[0 0.04977 0.1714] Hide interact prompt when the player stops being near the object
        (if (Utilities|Enum|Equal(Enum) (Variables|Default|GetMenuCheck) "NewEnumerator1")
          (Class|BPIHUD|BuildMenu(Message) _returnvalue false)
          (elif (Utilities|Enum|Equal(Enum) (Variables|Default|GetMenuCheck) "NewEnumerator2")
            (Class|BPIHUD|UpgradeMenu(Message) _returnvalue false (Variables|Default|GetLastSelectedTower))
            (elif (Utilities|Enum|Equal(Enum) (Variables|Default|GetMenuCheck) "NewEnumerator4")
              (Class|BPIHUD|ShopMenu(Message) _returnvalue false))))
        (Class|BPIHUD|InteractPrompt(Message) _returnvalue false) ; Hide the interact prompt and close the build menu
        (Variables|Default|SetMenuCheck "NewEnumerator3")))))

(event EventBeginPlay
  ;[0.1714 0 0.02843] Add mapping context
  (CallFunction|FuncSetValues)
  (CallFunction|FuncMappingContext)
  (Utilities|Time|SetTimerbyEvent (delegate Custom|CheckFloor) 0.05 true)
  (Variables|Default|SetKataneRotation (Variables|/Script/Engine.SceneComponent|GetRelativeRotation (Variables|Default|GetKatana))))

(event EventInteractPrompt
  (params (Valid :type Boolean))
  ;[0.05663 0.1771 0.01821] Change interact event
  (Variables|Default|SetMenuCheck "NewEnumerator3"))

(event EventUpdateStamina
  ;[0 0.05127 0.1559] Replenish Stamina slowly after not performing an action
  (Utilities|FlowControl|RetriggerableDelay 1.0)
  (bind _returnvalue (Utilities|Time|SetTimerbyEvent (delegate Custom|StaminaRegen) 0.025 true)))

(event EventTraceAgain
  (bind _selectedactor_s_ (Variables|Default|GetSelectedActor%28s%29))
  (bind _mesh (Variables|Character|GetMesh))
  (bind _selectedtag (Variables|Default|GetSelectedTag))
  (bind _returnvalue (Transformation|GetWorldLocation _mesh))
  ;[0.11 0 0] Interact with object
  (bind (_outhit _returnvalue_2) (Collision|CapsuleTraceByChannel _returnvalue _returnvalue (Variables|Default|GetInteract%20Radius) 0.0 "TraceTypeQuery3" false 0 "ForDuration" true "(R=1.000000,G=0.000000,B=0.000000,A=1.000000)" "(R=0.000000,G=1.000000,B=0.000000,A=1.000000)" 1.0))
  ;;[0.2874 0.1413 0.0137] Interact with building spot to build a tower
  (if _returnvalue_2 ; Necessary check to prevent compile error
    (if (and (.bblockinghit _outhit) (Actor|ActorHasTag (.hitactor _outhit) "Build"))
      (bind _output_get (Variables|Default|SetOut%20Hit%20Hit%20Actor (.hitactor _outhit)))
      (Utilities|Array|SetArrayElem (Variables|Default|GetSelectedActor%28s%29) 0 _output_get) ; Building Spot
      (Utilities|Array|SetArrayElem _selectedtag 0 (Utilities|Array|Get(acopy) (Variables|/Script/Engine.Actor|GetTags (Variables|Default|GetOut%20Hit%20Hit%20Actor)) 2)) ; On path or not
      (Variables|Default|SetMenuCheck "NewEnumerator1")
      (Class|BPIHUD|BuildMenu(Message) (Game|GetGameMode) true)
      (CallFunction|FuncCenterMouse))
    ;;[0.3372 0.1746 0.1329] Manage tower to upgrade or sell
    (if (and (.bblockinghit _outhit) (Actor|ActorHasTag (.hitactor _outhit) "Tower"))
      (bind _output_get_2 (Variables|Default|SetOut%20Hit%20Hit%20Actor (.hitactor _outhit)))
      (bind _outactors (Actor|GetAllActorsOfClass "/Game/Player/Blueprints/Gameplay/Actor_BuildSpot.Actor_BuildSpot_C"))
      (Utilities|Array|SetArrayElem _selectedactor_s_ 0 (.ReturnValue (Actor|FindNearestActor (Transformation|GetActorLocation _output_get_2) _outactors))) ; Building Spot
      (Utilities|Array|SetArrayElem _selectedactor_s_ 1 (Variables|Default|GetOut%20Hit%20Hit%20Actor)) ; Set tower to upgrade
      (Utilities|Array|SetArrayElem _selectedtag 1 (Utilities|Array|Get(acopy) (Variables|/Script/Engine.Actor|GetTags (Variables|Default|GetOut%20Hit%20Hit%20Actor)) 4)) ; SellPrice
      (Variables|Default|SetMenuCheck "NewEnumerator2")
      (bind _output_get_3 (Variables|Default|SetLastSelectedTower (Utilities|Array|Get(acopy) (Variables|/Script/Engine.Actor|GetTags (Variables|Default|GetOut%20Hit%20Hit%20Actor)) 3)))
      (Class|BPIHUD|UpgradeMenu(Message) (Game|GetGameMode) true _output_get_3)
      (CallFunction|FuncCenterMouse))
    ;;[0.05127 0.02732 0.0319] Open up the shop menu to buy useful items
    (if (and (.bblockinghit _outhit) (Actor|ActorHasTag (.hitactor _outhit) "Shop"))
      (Variables|Default|SetMenuCheck "NewEnumerator4")
      (Class|BPIHUD|ShopMenu(Message) (Game|GetGameMode) true)
      (CallFunction|FuncCenterMouse))
    (else
      (Class|BPIHUD|UseConsume(Message) (Game|GetGameMode)))))

(fn ConstructionScript)

(fn FuncMappingContext
  (bind _asplayer_ctrl_defense (Utilities|Casting|CastToPlayerCtrl_Defense (Pawn|GetController)))
  (Utilities|IsValid (PlayerController|LocalPlayerSubsystems|GetEnhancedInputLocalPlayerSubsystem _asplayer_ctrl_defense)
    (:Is%20Valid
      (Input|AddMappingContext (PlayerController|LocalPlayerSubsystems|GetEnhancedInputLocalPlayerSubsystem _asplayer_ctrl_defense) "/Game/Player/Input/InputMap_Defense.InputMap_Defense" 0 "(bIgnoreAllPressedKeysUntilRelease=True,bForceImmediately=False)"))))

(fn FuncCheckFloor)

(fn FuncStaminaRegen
  (params (Handle :type Timer%20Handle%20Structure%20%28by%20ref%29))
  (if (or (not (Variables|Default|GetValidDash)) (Variables|Default|GetSprinting)) ; when the player does an action, invalidate the timer used to trigger this function
    (Utilities|Time|ClearandInvalidateTimerbyHandle Handle)
    (elif (not (and (Variables|Default|GetValidDash) (Variables|Default|GetSprinting))) ; If the player is not doing a specified action
      (Variables|Default|SetStamina (Math|Float|Clamp(Float) (+ (Variables|Default|GetStamina) 0.01)))
      (Class|BPIHUD|UpdateStamina(Message) (Game|GetGameMode)))))

(fn FuncConsumeStamina
  (params (Amount :type Float%20%28double-precision%29))
  (Variables|Default|SetStamina (- (Variables|Default|GetStamina) Amount))
  (Class|BPIHUD|UpdateStamina(Message) (Game|GetGameMode)) ; Update HUD element
  (CallFunction|UpdateStamina))

(fn FuncSetValues
  (bind _charactermovement (Variables|Character|GetCharacterMovement))
  (bind _speed (Variables|Default|GetSpeed))
  (Variables|/Script/Engine.CharacterMovementComponent|SetMaxWalkSpeed _charactermovement _speed)
  (Variables|/Script/Engine.CharacterMovementComponent|SetMaxAcceleration _charactermovement (* _speed 4.0))
  (Components|Sphere|SetSphereRadius (Variables|Default|GetInteractRadius) (Variables|Default|GetInteract%20Radius) true)
  (Variables|/Script/Engine.SpringArmComponent|SetTargetArmLength (Variables|Default|GetSpringArm) (Variables|Default|GetTarget%20Arm%20Length))
  (Variables|Default|SetCurrentHealth (Variables|Default|GetMaxHealth)))

(fn FuncCenterMouse
  (bind _returnvalue (Viewport|GetViewportSize))
  (bind _returnvalue_2 (/ _returnvalue "(X=2.000000,Y=2.000000)"))
  (Class|PlayerController|SetMouseLocation (Game|GetPlayerController 0) (Math|Float|Truncate (.x _returnvalue_2)) (Math|Float|Truncate (.y _returnvalue_2))) ; set mouse cursor to the center of the viewport
)

(fn FuncSetWeaponVisibility
  (switch Utilities|FlowControl|Switch|SwitchonEnum_EquippedItem (Variables|Default|GetCurrentItem)
    (:NewEnumerator0
      (Rendering|SetVisibility (Variables|Default|GetKataneUnequipped) false true)
      (Rendering|SetVisibility (Variables|Default|GetKatana) true true)
      (Rendering|SetVisibility (Variables|Default|GetBowUnequipped) true true)
      (Rendering|SetVisibility (Variables|Default|GetBow) false false)
      (Rendering|SetVisibility (Variables|Default|GetMusketUnequipped) true true)
      (Rendering|SetVisibility (Variables|Default|GetMusket) false true))
    (:NewEnumerator1
      (Rendering|SetVisibility (Variables|Default|GetBowUnequipped) false true)
      (Rendering|SetVisibility (Variables|Default|GetBow) true false)
      (Rendering|SetVisibility (Variables|Default|GetKataneUnequipped) true true)
      (Rendering|SetVisibility (Variables|Default|GetKatana) false true)
      (Rendering|SetVisibility (Variables|Default|GetMusketUnequipped) true true)
      (Rendering|SetVisibility (Variables|Default|GetMusket) false true))
    (:NewEnumerator2
      (Rendering|SetVisibility (Variables|Default|GetMusketUnequipped) false true)
      (Rendering|SetVisibility (Variables|Default|GetMusket) true true)
      (Rendering|SetVisibility (Variables|Default|GetKataneUnequipped) true true)
      (Rendering|SetVisibility (Variables|Default|GetKatana) false true)
      (Rendering|SetVisibility (Variables|Default|GetBowUnequipped) true true)
      (Rendering|SetVisibility (Variables|Default|GetBow) false false)))
  (return))

(fn FuncMusketShot
  (Audio|PlaySoundatLocation "/Game/StarterContent/Audio/Explosion01.Explosion01" (Transformation|GetWorldLocation (Variables|Default|GetMusket)) "0, 0, 0" 0.05 1.5 0.0 0 0 0 0)
  (LocalVariables|SetLocalCameraLocation (Transformation|GetWorldLocation (Variables|Default|GetCamera)))
  (bind (_outhit _returnvalue) (Collision|CapsuleTraceByChannel (LocalVariables|GetLocalCameraLocation) (+ (LocalVariables|GetLocalCameraLocation) (* (Math|Vector|GetForwardVector (Camera|GetCameraRotation (Game|GetPlayerCameraManager 0))) (LocalVariables|GetTraceLength))) 25.0 0.0 "TraceTypeQuery2" false 0 "ForDuration"))
  (Utilities|IsValid (.hitactor _outhit)
    (:Is%20Valid
      (if (and (Actor|ActorHasTag (.hitactor _outhit) "Enemy") _returnvalue)
        (if (== (.hitbonename _outhit) "head")
          (LocalVariables|SetDamageDone (LocalVariables|GetHeadShotDamage))
          (else
            (LocalVariables|SetDamageDone (LocalVariables|GetBodyShotDamage))))
        (Game|Damage|ApplyDamage (.hitactor _outhit) (LocalVariables|GetDamageDone) 0 self "/Script/Engine.DamageType")
        (return)))))

(fn FuncBowAttack
  (if (Variables|Default|GetZoomedIn)
    (LocalVariables|SetShoothing? true)
    (bind _returnvalue (CallFunction|FuncCalculateArrow))
    (Game|SpawnActorfromClass "/Game/AI/BP/BP_Arrow.BP_Arrow_C" _returnvalue "Undefined" 0 0)))

(fn FuncCalculateArrow
  (bind _arrowspawn (Variables|Default|GetArrowSpawn))
  (bind _returnvalue (Transformation|GetWorldLocation _arrowspawn))
  (LocalVariables|SetLocalCameraLoc (Transformation|GetWorldLocation (Variables|Default|GetCamera)))
  (bind (_outhit _returnvalue_2) (Collision|LineTraceByChannel (LocalVariables|GetLocalCameraLoc) (+ (LocalVariables|GetLocalCameraLoc) (* (Math|Vector|GetForwardVector (Camera|GetCameraRotation (Game|GetPlayerCameraManager 0))) (LocalVariables|GettraceLength))) "TraceTypeQuery2" false 0 "None"))
  (if _returnvalue_2
    (return (Math|Transform|MakeTransform _returnvalue (Math|Rotator|FindLookatRotation _returnvalue (.ImpactPoint (Collision|BreakHitResult _outhit)))))
    (else
      (return (Math|Transform|MakeTransform _returnvalue (Math|Rotator|FindLookatRotation _returnvalue (+ (LocalVariables|GetLocalCameraLoc) (* (Math|Vector|GetForwardVector (Camera|GetCameraRotation (Game|GetPlayerCameraManager 0))) (LocalVariables|GettraceLength)))))))))

(fn UseAmmo
  (params (Weapon :type Enum_EquippedItem%20Enum :default "NewEnumerator0")))