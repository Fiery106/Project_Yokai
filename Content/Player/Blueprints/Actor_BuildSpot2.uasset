(event EventBeginPlay
  (CallFunction|FuncHideObject true)
  (if (Variables|Default|GetOnPath)
    (Utilities|Array|SetArrayElem (Variables|Actor|GetTags) 2 "Path")))

(event EventConstruct
  (params (TowerToBuild :type Enum_Towers%20Enum :default "NewEnumerator0"))
  (if (not (Variables|Default|GetOccupied))
    (Variables|Default|SetOccupied true)
    (CallFunction|FuncHideObject false)))

(event EventSell
  (Variables|Default|SetOccupied false)
  (CallFunction|FuncHideObject true)
  (bind _outactors (Actor|GetAllActorsOfClass "/Game/Towers/Actor_Tower.Actor_Tower_C"))
  (if (not (> (.Distance (Actor|FindNearestActor (Transformation|GetActorLocation) _outactors)) 0.0))
    (Actor|DestroyActor (.ReturnValue (Actor|FindNearestActor (Transformation|GetActorLocation) _outactors)))))

(fn ConstructionScript)

(fn FuncHideObject
  (params (Visible :type Boolean))
  (bind _cube (Variables|Default|GetCube))
  (if Visible
    (Rendering|SetVisibility _cube true false)
    (Collision|SetCollisionEnabled _cube "QueryAndPhysics")
    (else
      (Rendering|SetVisibility _cube false false)
      (Collision|SetCollisionEnabled _cube "NoCollision"))))